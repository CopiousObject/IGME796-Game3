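; DogLaughing is an actor that pops up and drops back down, apparently the laughing dog between targets in a VR shooting game.
; Tick adds VerticalMod to its Z each frame without delta-time scaling, pausing at height 230 until a one-second timer sets a downward speed.
; Once below -10 it destroys itself and calls SpawnTarget on VRGameMode.
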(event Custom|SetVerticalMod
  (Variables|Default|SetVerticalMod -1e+01))

(event EventBeginPlay)

(event Collision|EventActorBeginOverlap
  (params (OtherActor :type Actor%20Object%20Reference)))

(event EventTick
  (params (DeltaSeconds :type Float%20%28single-precision%29))
  (bind _returnvalue (Transformation|GetActorLocation))
  (if (Variables|Default|GetMoving%20Down)
    (Transformation|SetActorLocation (Math|Vector|MakeVector (.x _returnvalue) (.y _returnvalue) (+ (.z _returnvalue) (Variables|Default|GetVerticalMod))) false false :!label _label)
    (if (< (.z _returnvalue) -1e+01)
      (Actor|DestroyActor)
      (bind _returnvalue_2 (Actor|GetActorOfClass "/Game/VRTemplate/Blueprints/VRGameMode.VRGameMode_C"))
      (Default|SpawnTarget _returnvalue_2))
    (elif (>= (.z _returnvalue) 2.3e+02)
      (Variables|Default|SetMoving%20Down true)
      (Variables|Default|SetVerticalMod 0.0)
      (Utilities|Time|SetTimerbyEvent (delegate Custom|SetVerticalMod) 1.0)
      (else
        (goto _label)))))

(fn ConstructionScript)