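; FallingTargets is a target actor that scores when it drops below a height threshold in what appears to be a VR game.
; Tick checks its height, destroys it below that floor and calls UpdateScore on the VRGameMode, fetched via GetActorOfClass.
; RandomDirection sets VerticalMod when Direction equals HorizontalMod, otherwise HorizontalMod, steering inward past bounds and randomizing within them.
; Nothing here calls that function or applies movement.
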(event EventTick
  (params (DeltaSeconds :type Float%20%28single-precision%29))
  (if (< (.z (Transformation|GetActorLocation)) 9e+01)
    (Actor|DestroyActor)
    (bind _returnvalue (Actor|GetActorOfClass "/Game/VRTemplate/Blueprints/VRGameMode.VRGameMode_C"))
    (Default|UpdateScore _returnvalue)))

(fn ConstructionScript)

(fn RandomDirection
  (params (Direction :type Float%20%28double-precision%29))
  (bind _returnvalue (Transformation|GetActorLocation))
  (if (== Direction (Variables|Default|GetHorizontalMod))
    (if (< (.z _returnvalue) 1.8e+02)
      (Variables|Default|SetVerticalMod 1.0)
      (elif (> (.z _returnvalue) 1.5e+03)
        (Variables|Default|SetVerticalMod -1.0)
        (else
          (Variables|Default|SetVerticalMod (Math|Conversions|ToFloat(Integer) (Math|Random|RandomIntegerinRange -1 1))))))
    (elif (< (.y _returnvalue) -1.44e+03)
      (Variables|Default|SetHorizontalMod 1.0)
      (elif (> (.y _returnvalue) 8e+02)
        (Variables|Default|SetHorizontalMod -1.0)
        (else
          (Variables|Default|SetHorizontalMod (Math|Conversions|ToFloat(Integer) (Math|Random|RandomIntegerinRange -1 1))))))))