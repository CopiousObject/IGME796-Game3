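; FallingTarg is a shot duck in a VR Duck Hunt-style game that pauses, then falls and brings up the dog.
; BeginPlay picks a sprite by the game mode's DuckColor, and a half-second timer swaps it and enables projectile gravity.
; Tick spins the sprite using VerticalMod and, below a height threshold, destroys the actor and spawns DogShowing at its X/Y.
; A RandomDirection function for bounded movement is defined but never called here.
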(event Custom|StartFall
  (Rendering|Components|Sprite|SetSprite (Variables|Default|GetPaperSprite) (Utilities|Array|Get(acopy) (Variables|Default|GetSprites) (+ (* (Variables|Default|GetBirdColor) 2) 1)))
  (Variables|/Script/Engine.ProjectileMovementComponent|SetProjectileGravityScale (Variables|Default|GetProjectileMovement) 1.0)
  (Variables|Default|SetVerticalMod -23.0))

(event EventTick
  (params (DeltaSeconds :type Float%20%28single-precision%29))
  (bind _returnvalue (Transformation|GetActorLocation))
  (Transformation|AddLocalRotation (Variables|Default|GetPaperSprite) (Math|Rotator|MakeRotator 0.0 0.0 (Variables|Default|GetVerticalMod)) false false)
  (if (< (.z _returnvalue) 9e+01)
    (Actor|DestroyActor)
    (Game|SpawnActorfromClass "/Game/Blueprints/DogShowing.DogShowing_C" (Math|Transform|MakeTransform (Math|Vector|MakeVector (.x _returnvalue) (.y _returnvalue) -1e+01) "0, 0, 0" "1.000000,1.000000,1.000000") "Undefined" "MultiplyWithRoot" 0 0)))

(event EventBeginPlay
  (bind _returnvalue (Actor|GetActorOfClass "/Game/VRTemplate/Blueprints/VRGameMode.VRGameMode_C"))
  (Variables|Default|SetBirdColor (Variables|/Game/VRTemplate/Blueprints/VRGameMode.VRGameMode_C|GetDuckColor _returnvalue))
  (Rendering|Components|Sprite|SetSprite (Variables|Default|GetPaperSprite) (Utilities|Array|Get(acopy) (Variables|Default|GetSprites) (* (Variables|Default|GetBirdColor) 2)))
  (Utilities|Time|SetTimerbyEvent (delegate Custom|StartFall) 0.5))

(fn ConstructionScript)

(fn RandomDirection
  (params (Direction :type Float%20%28double-precision%29))
  (bind _returnvalue (Transformation|GetActorLocation))
  (if (== Direction (Variables|Default|GetHorizontalMod))
    (if (< (.z _returnvalue) 1.8e+02)
      (Variables|Default|SetVerticalMod 1.0)
      (elif (> (.z _returnvalue) 1.5e+03)
        (Variables|Default|SetVerticalMod -1.0)
        (else
          (Variables|Default|SetVerticalMod (Math|Conversions|ToFloat(Integer) (Math|Random|RandomIntegerinRange -1 1))))))
    (elif (< (.y _returnvalue) -1.44e+03)
      (Variables|Default|SetHorizontalMod 1.0)
      (elif (> (.y _returnvalue) 8e+02)
        (Variables|Default|SetHorizontalMod -1.0)
        (else
          (Variables|Default|SetHorizontalMod (Math|Conversions|ToFloat(Integer) (Math|Random|RandomIntegerinRange -1 1))))))))