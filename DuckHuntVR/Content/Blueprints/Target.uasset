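; Duck target for a VR Duck Hunt-style game that flies erratically in the Y/Z plane, with random color and game-mode speed.
; A looping timer, faster in later rounds, rerolls bounded horizontal and vertical directions, which Tick applies as movement.
; SpriteManager selects the color's flipbook for horizontal, vertical or diagonal flight and mirrors it by rotation.
; After about ten seconds it escapes upward, destroys itself and spawns DogLaughing.
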(event Custom|SetMovement
  (bind _returnvalue (Math|Random|RandomBool))
  (Variables|Default|SetMaxTime (+ (Variables|Default|GetMaxTime) (Variables|Default|GetTimeMod)))
  (CallFunction|RandomDirection (Variables|Default|GetHorizontalMod))
  (if (>= (Variables|Default|GetMaxTime) 1e+01)
    (Variables|Default|SetVerticalMod 1.0)
    (CallFunction|SpriteManager :!label _label)
    (else
      (CallFunction|RandomDirection (Variables|Default|GetVerticalMod))
      (if (and (== (Variables|Default|GetHorizontalMod) 0.0) (== (Variables|Default|GetVerticalMod) 0.0))
        (if (Math|Random|RandomBool)
          (if _returnvalue
            (Variables|Default|SetVerticalMod 1.0)
            (else
              (Variables|Default|SetVerticalMod -1.0)))
          (elif _returnvalue
            (Variables|Default|SetHorizontalMod 1.0)
            (else
              (Variables|Default|SetHorizontalMod -1.0))))
        (CallFunction|SpriteManager)
        (else
          (goto _label))))))

(event EventBeginPlay
  (bind _output_get (Variables|Default|SetBirdColor (Math|Random|RandomInteger 3)))
  (bind _returnvalue (Actor|GetActorOfClass "/Game/VRTemplate/Blueprints/VRGameMode.VRGameMode_C"))
  (Variables|/Game/VRTemplate/Blueprints/VRGameMode.VRGameMode_C|SetDuckColor _returnvalue _output_get)
  (Variables|Default|SetSpeed (Variables|/Game/VRTemplate/Blueprints/VRGameMode.VRGameMode_C|GetSpeed _returnvalue))
  (if (< (Variables|/Game/VRTemplate/Blueprints/VRGameMode.VRGameMode_C|GetRound%20Count _returnvalue) 11)
    (Variables|Default|SetTimeMod (Math|Float|Power 0.9 (Math|Conversions|ToFloat(Integer) (- (Variables|/Game/VRTemplate/Blueprints/VRGameMode.VRGameMode_C|GetRound%20Count _returnvalue) 1)))))
  (Variables|Default|SetHorizontalMod (Math|Conversions|ToFloat(Integer) (Math|Random|RandomIntegerinRange -1 1)))
  (CallFunction|SpriteManager)
  (Utilities|Time|SetTimerbyEvent (delegate Custom|SetMovement) (Variables|Default|GetTimeMod) true))

(event Collision|EventActorBeginOverlap
  (params (OtherActor :type Actor%20Object%20Reference)))

(event EventTick
  (params (DeltaSeconds :type Float%20%28single-precision%29))
  (bind _returnvalue (Transformation|GetActorLocation))
  (if (>= 1e+01 (Variables|Default|GetMaxTime))
    (Transformation|SetActorLocation (Math|Vector|MakeVector (.x _returnvalue) (+ (* (Variables|Default|GetSpeed) (Variables|Default|GetHorizontalMod)) (.y _returnvalue)) (+ (.z _returnvalue) (* (Variables|Default|GetSpeed) (Variables|Default|GetVerticalMod)))) false false :!label _label)
    (if (< (+ (.z _returnvalue) (* (Variables|Default|GetSpeed) (Variables|Default|GetVerticalMod))) 1.8e+02)
      (Variables|Default|SetVerticalMod 1.0)
      (CallFunction|SpriteManager))
    (elif (< (.z (Transformation|GetActorLocation)) 1.8e+03)
      (goto _label)
      (else
        (Actor|DestroyActor)
        (Game|SpawnActorfromClass "/Game/Blueprints/DogLaughing.DogLaughing_C" (Math|Transform|MakeTransform "-4750.000000,-292.967614,-10.000000" "0, 0, 0" "1.000000,1.000000,1.000000") "Undefined" "MultiplyWithRoot" 0 0)))))

(fn ConstructionScript)

(fn RandomDirection
  (params (Direction :type Float%20%28double-precision%29))
  (bind _returnvalue (Transformation|GetActorLocation))
  (if (== Direction (Variables|Default|GetHorizontalMod))
    (if (< (.z _returnvalue) 1.8e+02)
      (Variables|Default|SetVerticalMod 1.0)
      (elif (> (.z _returnvalue) 1.5e+03)
        (Variables|Default|SetVerticalMod -1.0)
        (else
          (Variables|Default|SetVerticalMod (Math|Conversions|ToFloat(Integer) (Math|Random|RandomIntegerinRange -1 1))))))
    (elif (< (.y _returnvalue) -1.44e+03)
      (Variables|Default|SetHorizontalMod 1.0)
      (elif (> (.y _returnvalue) 8e+02)
        (Variables|Default|SetHorizontalMod -1.0)
        (else
          (Variables|Default|SetHorizontalMod (Math|Conversions|ToFloat(Integer) (Math|Random|RandomIntegerinRange -1 1))))))))

(fn SpriteManager
  (bind _spritesheet (Variables|Default|GetSpriteSheet))
  (bind _verticalmod (Variables|Default|GetVerticalMod))
  (bind _horizontalmod (Variables|Default|GetHorizontalMod))
  (if (!= (Variables|Default|GetVerticalMod) 0.0) ; If vertical mod is zero
    (if (== (Variables|Default|GetHorizontalMod) 0.0) ; In the case that it VerticalMod is not zero\n\nIs the horizontal mod zero
      (Sprite|SetFlipbook (Variables|Default|GetSpriteSheet) (Utilities|Array|Get(acopy) (Variables|Default|GetSprites) (+ (* (Variables|Default|GetBirdColor) 3) 2))) ; Bird must be flying vertically
      (Transformation|SetRelativeRotation _spritesheet (Math|Rotator|MakeRotator 0.0 (* (+ 9e+01 (* -9e+01 _verticalmod)) (Math|Float|Absolute(Float) _verticalmod)) (* (Math|Float|Absolute(Float) _horizontalmod) (+ (* _horizontalmod -9e+01) 9e+01))) false false :!label _label)
      (else
        (Sprite|SetFlipbook (Variables|Default|GetSpriteSheet) (Utilities|Array|Get(acopy) (Variables|Default|GetSprites) (* (Variables|Default|GetBirdColor) 3))) ; Bird must be flying diagonally
        (if (== (Variables|Default|GetHorizontalMod) -1.0)
          (if (== (Variables|Default|GetVerticalMod) -1.0)
            (Transformation|SetRelativeRotation _spritesheet "180.000000,0.000000,0.000000" false false)
            (else
              (Transformation|SetRelativeRotation _spritesheet "0.000000,180.000000,0.000000" false false)))
          (elif (== (Variables|Default|GetVerticalMod) -1.0)
            (Transformation|SetRelativeRotation _spritesheet "180.000000,180.000000,0.000000" false false)
            (else
              (Transformation|SetRelativeRotation _spritesheet "0, 0, 0" false false))))))
    (else
      (Sprite|SetFlipbook (Variables|Default|GetSpriteSheet) (Utilities|Array|Get(acopy) (Variables|Default|GetSprites) (+ (* (Variables|Default|GetBirdColor) 3) 1))) ; Bird must be flying horizontally
      (goto _label))))